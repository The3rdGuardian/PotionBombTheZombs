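; BP_Zombear is a Zombear actor with hit points and a floating health readout.
; The ModHP event subtracts the given value from HP, then destroys the actor below 1 or writes the new value to the Health text.
; Each tick rotates the Health text to face the player camera manager's location, billboard style.
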(event EventTick
  (params (DeltaSeconds :type Float%20%28single-precision%29))
  (Transformation|SetWorldRotation (Variables|Default|GetHealth) (Math|Rotator|MakeRotationfromAxes (- (Transformation|GetActorLocation (Game|GetPlayerCameraManager 0)) (Transformation|GetActorLocation)) "0, 0, 0" "0, 0, 0") false false))

(event EventModHP
  (params (ModValue :type Integer))
  (bind _output_get (Variables|Default|SetHP (- (Variables|Default|GetHP) ModValue)))
  (if (< _output_get 1)
    (Actor|DestroyActor)
    (else
      (Rendering|Components|TextRender|SetText (Variables|Default|GetHealth) (Utilities|Text|ToText(Integer) _output_get)))))

(fn ConstructionScript)