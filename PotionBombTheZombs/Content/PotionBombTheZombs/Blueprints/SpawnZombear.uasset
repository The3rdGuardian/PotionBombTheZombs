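; SpawnZombear is a wave spawner that creates BP_Zombear AI enemies at the location of its Spawn component.
; On BeginPlay, the WaveSpawn timeline fires Wave events, each spawning one Zombear regardless of collision.
; If that newly spawned Zombear's IsDestroyed value equals eight, a short delay starts a second timeline whose Wave events spawn further Zombears at the same point.
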(event EventBeginPlay
  (Timeline|Wave%20Spawn Play
    (:Wave
      (bind _returnvalue (AI|SpawnAIFromClass "/Game/PotionBombTheZombs/Blueprints/BP_Zombear.BP_Zombear_C" 0 (Transformation|GetWorldLocation (Variables|Default|GetSpawn)) "0.000000,-90.000000,0.000000" true 0))
      (bind _asbp_zombear (Utilities|Casting|CastToBP_Zombear _returnvalue))
      (if (== (Variables|/Game/PotionBombTheZombs/Blueprints/BP_Zombear.BP_Zombear_C|GetisDestroyed _asbp_zombear) 8)
        (Utilities|FlowControl|Delay 3.0)
        (Timeline|Timeline_0 Play
          (:Wave
            (AI|SpawnAIFromClass "/Game/PotionBombTheZombs/Blueprints/BP_Zombear.BP_Zombear_C" 0 (Transformation|GetWorldLocation (Variables|Default|GetSpawn)) "0.000000,-90.000000,0.000000" true 0)))))))

(fn ConstructionScript)